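; Tank projectile Blueprint that handles the shell's firing sound and in-flight audio.
; On BeginPlay it plays a randomized mortar sound and records distance to the player pawn, destroying the flight audio for launches under 1000 units.
; While EnemyTank is set, Tick scales volume and pitch by camera distance relative to launch distance, lowering both as the shell nears.
; A collision hit stops the audio and updates.
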(event `self.ReceiveBeginPlay`
  ;[1 1 1] Get total fly distance at fire
  (bind _output_get (set `self.LaunchDistance` (`self.GetDistanceTo` (`GameplayStatics.GetPlayerPawn` 0))))
  (bind _returnvalue (>= _output_get 1000.0))
  (`KismetSystemLibrary.PrintString` (`KismetStringLibrary.Conv_BoolToString` _returnvalue))
  (if (not _returnvalue)
    ;[1 1 1] If launch distance is less than 20 meters, no audio
    (set `self.EnemyTank` false)
    (`ActorComponent.K2_DestroyComponent` (`self.Audio`)))
  ;[1 1 1] Play firing sound
  (`GameplayStatics.PlaySoundAtLocation` "/Game/Mortar_Round-SoundBible_com-1560834884.Mortar_Round-SoundBible_com-1560834884" (`self.K2_GetActorLocation`) (struct) 1.0 (`KismetMathLibrary.RandomFloatInRange` 0.95 1.15) (`KismetMathLibrary.RandomFloatInRange` 0.0 0.5)))

(event `self.ReceiveTick`
  (params (DeltaSeconds :type "Float (single-precision)"))
  (bind _audio (`self.Audio`))
  (bind _returnvalue (`KismetMathLibrary.Lerp` 0.0 2.0 (/ (`self.GetDistanceTo` (`GameplayStatics.GetPlayerCameraManager` 0)) (`self.LaunchDistance`))))
  (if (`self.EnemyTank`)
    (`KismetSystemLibrary.PrintString` (`KismetStringLibrary.Conv_DoubleToString` _returnvalue))
    (`AudioComponent.SetVolumeMultiplier` _audio _returnvalue)
    (`AudioComponent.SetPitchMultiplier` _audio _returnvalue)))

(event `self.CollisionMesh.OnComponentHit`
  (params (HitComponent :type "PrimitiveComponent Object Reference") (OtherActor :type "Actor Object Reference") (OtherComp :type "PrimitiveComponent Object Reference") (NormalImpulse :type "Vector Structure") (Hit :type "HitResult Structure (by ref)"))
  ;[1 1 1] Projectile exploded. Stop audio
  (`AudioComponent.Stop` (`self.Audio`))
  (set `self.EnemyTank` false))

(fn `UserConstructionScript`)